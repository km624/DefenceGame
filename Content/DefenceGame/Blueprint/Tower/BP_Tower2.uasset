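; Defence-game tower Blueprint that drives an attached option widget for upgrading and removing the tower.
; On BeginPlay it caches the BP_TowerOptBtn widget, shows the next upgrade cost and binds its remove and level-up buttons.
; OptionWidget toggles the options and debug flag, slowing global time while they are open.
; Successful TowerLevelUp calls add a BP_StartWidget to the level box and update the cost, showing MAX when it reaches zero.
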(event Custom|LevelUp
  (bind _nextleveltowermoney (Variables|Default|GetNextLevelTowerMoney))
  (bind _toweroptbtn (Variables|Default|GetTowerOptBtn))
  (bind _textblock_money (Variables|/Game/DefenceGame/Blueprint/UI/BP_TowerOptBtn.BP_TowerOptBtn_C|GetTextBlock_Money _toweroptbtn))
  (bind _returnvalue (Class|TowerDefenceGameCharacter|TowerLevelUp (Variables|Default|GetCurrentLevel)))
  (if _returnvalue
    (bind _returnvalue_2 (UserInterface|CreateWidget "/Game/DefenceGame/Blueprint/UI/BP_StartWidget.BP_StartWidget_C"))
    (Widget|Panel|AddChild (Variables|/Game/DefenceGame/Blueprint/UI/BP_TowerOptBtn.BP_TowerOptBtn_C|GetHorizontalBox_LevelBox (Variables|Default|GetTowerOptBtn)) _returnvalue_2)
    (if (== _nextleveltowermoney 0.0)
      (Rendering|Components|TextRender|SetText _textblock_money "MAX")
      (Widget|SetVisibility (Variables|/Game/DefenceGame/Blueprint/UI/BP_TowerOptBtn.BP_TowerOptBtn_C|GetTextBlock_Minus _toweroptbtn) "Hidden")
      (else
        (Rendering|Components|TextRender|SetText _textblock_money (Utilities|Text|ToText(Float) _nextleveltowermoney "HalfToEven"))))))

(event Custom|DsetroyTower
  (Class|TowerDefenceGameCharacter|TowerRemove)
  (Utilities|Time|SetGlobalTimeDilation 1.0))

(event EventBeginPlay
  (bind _asbp_tower_opt_btn (Utilities|Casting|CastToBP_TowerOptBtn (UserInterface|GetWidget (Variables|Default|GetWidget)))
    (:then
      (Rendering|Components|TextRender|SetText (Variables|/Game/DefenceGame/Blueprint/UI/BP_TowerOptBtn.BP_TowerOptBtn_C|GetTextBlock_Money _asbp_tower_opt_btn) (Utilities|Text|ToText(Float) (Variables|Default|GetNextLevelTowerMoney) "HalfToEven"))
      (bind _output_get (Variables|Default|SetTowerOptBtn _asbp_tower_opt_btn))
      (EventDispatchers|AssignOnClicked (Variables|/Game/DefenceGame/Blueprint/UI/BP_TowerOptBtn.BP_TowerOptBtn_C|GetButton_Remove _output_get) (delegate Custom|DsetroyTower))
      (EventDispatchers|BindEventtoOnClicked (Variables|/Game/DefenceGame/Blueprint/UI/BP_TowerOptBtn.BP_TowerOptBtn_C|GetButton_LevelUp _output_get) (delegate Custom|LevelUp)))
    (:CastFailed
      (Development|PrintString "Failed"))))

(event EventOptionWidget
  (bind _toweroptbtn (Variables|Default|GetTowerOptBtn))
  (bind _horizontalbox_toweroption (Variables|/Game/DefenceGame/Blueprint/UI/BP_TowerOptBtn.BP_TowerOptBtn_C|GetHorizontalBox_TowerOption _toweroptbtn))
  (if (Utilities|Enum|Equal(Enum) (Widget|GetVisibility _horizontalbox_toweroption) "Hidden")
    (Widget|SetVisibility _horizontalbox_toweroption "Visible")
    (Variables|Default|SetShowDebug true)
    (Utilities|Time|SetGlobalTimeDilation 0.2)
    (else
      (Widget|SetVisibility _horizontalbox_toweroption "Hidden")
      (Variables|Default|SetShowDebug false)
      (Utilities|Time|SetGlobalTimeDilation 1.0))))

(fn ConstructionScript)